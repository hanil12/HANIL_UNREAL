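; BP_MyGameInstance is a Game Instance that provides character stat data by level from a DataTable.
; On Init, it assigns BP_MyCharacterStatTable as the DataTable if none is valid.
; GetStatDataByLevel converts the level number into a row name and returns the matching row, printing a message when no row is found.
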(event `self.ReceiveInit`
  ;[1 1 1] Set DataTable
  (if (not (`KismetSystemLibrary.IsValid` (`self.DataTable`)))
    (set `self.DataTable` "/Game/Data/BP_MyCharacterStatTable.BP_MyCharacterStatTable")))

(fn `GetStatDataByLevel`
  (params (level :type Integer))
  (returns (NewParam :type "/Game/BluePrints/BPOnly/MyCharacterData Structure"))
  ;[1 1 1] Level로 StatData찾기
  (bind _returnvalue (`|GetDataTableRow` (`self.DataTable`) (`KismetStringLibrary.Conv_StringToName` (`KismetStringLibrary.Conv_IntToString` level)))
    (:`then`
      (return _returnvalue))
    (:`RowNotFound`
      (`KismetSystemLibrary.PrintString` "Not Found Stat Data by Level"))))